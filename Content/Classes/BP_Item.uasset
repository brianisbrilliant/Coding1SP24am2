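; BP_Item is an item actor with a name, type and damage, and stubbed pickup, drop and use events.
; On BeginPlay it calls Constructor, prints its name and damage, waits briefly, then Attack subtracts Damage from a found BP__enemy's Health.
; Constructor only sets the cube's material slot.
; Its type-based damage and random weapon naming logic is disconnected, and the Construction Script is empty.
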(event `self.ReceiveBeginPlay`
  (`self.Constructor`)
  (`KismetSystemLibrary.PrintString` (`KismetStringLibrary.Concat_StrStr` "Name: " (`self.Name`) ", Damage: " (`KismetStringLibrary.Conv_IntToString` (`self.Damage`))) true true (struct :`G` 0.66 :`B` 1.0 :`A` 1.0) 5.0)
  (`KismetSystemLibrary.Delay` 5.0)
  (bind _returnvalue (`GameplayStatics.GetActorOfClass` "/Game/Classes/BP__enemy.BP__enemy_C"))
  (`self.Attack` _returnvalue))

(event `pickup`)

(event `Drop`)

(event `Use`)

(fn `Attack`
  (params (GivenEnemy :type "/Game/Classes/BP__enemy Object Reference"))
  (set `/Game/Classes/BP__enemy.health` (- (`/Game/Classes/BP__enemy.health` GivenEnemy) (`self.Damage`)) GivenEnemy) ; set health
)

(fn `Constructor`
  (`PrimitiveComponent.SetMaterial` (`self.Cube`) 0 null))

(fn `UserConstructionScript`)